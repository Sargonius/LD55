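; BP_MovableBackground is a background prop actor that scrolls continuously and loops back to create endless moving scenery.
; Its construction script calls Generate, which picks a random mesh from MeshVariants and applies the set scale and a random rotation.
; Tick moves it along its forward vector by Speed, scaled to a 60 fps baseline, and wraps its X position to the far positive side once it passes the negative limit.
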(event `Generate`
  (`StaticMeshComponent.SetStaticMesh` (`self.StaticMesh`) (`KismetArrayLibrary.Array_Random` (`self.MeshVariants`)))
  (`SceneComponent.SetRelativeScale3D` (`self.StaticMesh`) (`self.Scale`))
  (`SceneComponent.K2_SetRelativeRotation` (`self.StaticMesh`) (`KismetMathLibrary.RandomRotator` false) false false))

(event `self.ReceiveTick`
  (params (DeltaSeconds :type "Float (single-precision)"))
  (bind (_returnvalue_x _returnvalue_y _returnvalue_z) (`KismetMathLibrary.BreakVector` (`self.K2_GetActorLocation`)))
  (`self.K2_AddActorWorldOffset` (* (`self.GetActorForwardVector`) (`self.Speed`) (* DeltaSeconds 60.0)))
  (if (< _returnvalue_x -5000.0)
    (`self.K2_SetActorLocation` (`KismetMathLibrary.MakeVector` 5000.0 _returnvalue_y _returnvalue_z))))

(fn `UserConstructionScript`
  (`self.Generate`))