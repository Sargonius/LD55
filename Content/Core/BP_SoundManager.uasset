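; BP_SoundManager switches the game's music from ambient to boss when the boss appears.
; On BeginPlay it plays the ambient track, stops the boss track and binds to the OnAppear event of the BP_Boss it finds in the level.
; When the boss appears, a Crossfade timeline blends the two tracks' volume multipliers.
; A CrossfadeFromBoss event reverses the timeline, though nothing in this Blueprint calls it.
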(event `self.ReceiveBeginPlay`
  (bind _returnvalue (`GameplayStatics.GetActorOfClass` "/Game/Blueprints/BP_Boss.BP_Boss_C"))
  (add `/Game/Blueprints/BP_Boss.OnAppear` _returnvalue (delegate `On Boss Appear`))
  (`AudioComponent.Play` (`self.Ambient`) 0.0)
  (`AudioComponent.Stop` (`self.Boss`)))

(event `On Boss Appear`
  (`AudioComponent.Play` (`self.Boss`) 0.0)
  (`self.Crossfade To Boss`))

(event `Crossfade To Boss`
  (bind (_direction _ambientmusic _bossmusic) (`Timeline|Crossfade` :!via `PlayFromStart` :!label _label)
    (:`Update`
      (`AudioComponent.SetVolumeMultiplier` (`self.Ambient`) _ambientmusic)
      (`AudioComponent.SetVolumeMultiplier` (`self.Boss`) _bossmusic))))

(event `Crossfade From Boss`
  (goto _label :!via `ReverseFromEnd`))

(fn `UserConstructionScript`)