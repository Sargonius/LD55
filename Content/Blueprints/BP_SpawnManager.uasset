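; BP_SpawnManager periodically spawns fish through a registry of spawners that register and unregister themselves.
; A looping timer, with its interval randomized once at BeginPlay, skips spawning when the BP_Fish count exceeds the cap.
; Otherwise it requests a batch scaled by the BP_Summoner count, without rechecking the cap.
; Each request picks randomly from active spawners, with separate picks for the validity check and spawn call.
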(event `Register Spawner`
  (params (InSpawner :type "/Game/Blueprints/BP_FishSpawner Object Reference"))
  (`KismetArrayLibrary.Array_AddUnique` (`self.ActiveSpawners`) InSpawner))

(event `Unregister Spawner`
  (params (InSpawner :type "/Game/Blueprints/BP_FishSpawner Object Reference"))
  (`KismetArrayLibrary.Array_RemoveItem` (`self.ActiveSpawners`) InSpawner))

(event `Spawn`
  (bind _outitem (`KismetArrayLibrary.Array_Random` (`self.ActiveSpawners`)))
  (`/Engine/EditorBlueprintResources/StandardMacros.IsValid` _outitem
    (:`Is Valid`
      (`/Game/Blueprints/BP_FishSpawner.Spawn` _outitem))))

(event `self.ReceiveBeginPlay`
  (`KismetSystemLibrary.K2_SetTimerDelegate` (delegate `Tick Spawn`) (`KismetMathLibrary.RandomFloatInRange` 2.0 4.0) true))

(event `Tick Spawn`
  (bind _outactors (`GameplayStatics.GetAllActorsOfClass` "/Game/Blueprints/BP_Fish.BP_Fish_C"))
  (if (not (> (`KismetArrayLibrary.Array_Length` _outactors) (`self.MaxFishToSpawn`)))
    (bind _outactors_2 (`GameplayStatics.GetAllActorsOfClass` "/Game/Blueprints/Summoners/BP_Summoner.BP_Summoner_C"))
    (for _ (range (* (`KismetArrayLibrary.Array_Length` _outactors_2) (`self.FishToSpawn`)))
      (`self.Spawn`))))

(fn `UserConstructionScript`)