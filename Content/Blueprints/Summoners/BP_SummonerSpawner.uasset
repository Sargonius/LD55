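; BP_SummonerSpawner periodically spawns summoners and triggers the boss appearance cinematic once every summoner location is used.
; BeginPlay gathers all BP_SummonerLocation actors and starts a looping timer with an interval randomized once.
; Each tick of the timer removes a random location and spawns a BP_Summoner at the spawner's transform, passing that location as its target.
; An empty list plays LS_BossAppearance through a DoOnce, though the timer keeps running.
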(event `Get All Summoner Spawners`
  (bind _outactors (`GameplayStatics.GetAllActorsOfClass` "/Game/Blueprints/Summoners/BP_SummonerLocation.BP_SummonerLocation_C"))
  (set `self.SummonerSpawners` _outactors))

(event `self.ReceiveBeginPlay`
  (`KismetSystemLibrary.K2_SetTimerDelegate` (delegate `Spawn Summoner`) (`KismetMathLibrary.RandomFloatInRange` 15.0 20.0) true)
  (`self.Get All Summoner Spawners`))

(event `Spawn Summoner`
  (bind _summonerspawners (`self.SummonerSpawners`))
  (bind _output_get (set `self.CurrentSpawn` (`KismetArrayLibrary.Array_Random` _summonerspawners)))
  (`KismetArrayLibrary.Array_RemoveItem` _summonerspawners _output_get)
  (`|SpawnActorFromClass` "/Game/Blueprints/Summoners/BP_Summoner.BP_Summoner_C" (`self.GetTransform`) "Undefined" "MultiplyWithRoot" null (`self.K2_GetActorLocation` _output_get) null)
  (if (`KismetArrayLibrary.Array_IsEmpty` _summonerspawners)
    (`/Engine/EditorBlueprintResources/StandardMacros.DoOnce` false
      (:`Completed`
        (`LevelSequencePlayer.CreateLevelSequencePlayer` "/Game/LS_BossAppearance.LS_BossAppearance" (make `MovieSceneSequencePlaybackSettings` true (struct) 1.0 0.0 false false false false false false false true))))))

(fn `UserConstructionScript`)