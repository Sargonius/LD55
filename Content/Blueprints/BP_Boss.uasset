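; BP_Boss is a boss actor that loses health when hit by first-person projectiles.
; Its Hit event ignores other actors, destroys the projectile, decrements Health and calls the OnHealthChanged dispatcher.
; When Health reaches zero or below, a DoOnce gate ensures the W_Victory widget is created for the first player and added to the viewport only once.
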(event `self.ReceiveHit`
  (params (MyComp :type "PrimitiveComponent Object Reference") (Other :type "Actor Object Reference") (OtherComp :type "PrimitiveComponent Object Reference") (bSelfMoved :type Boolean) (HitLocation :type "Vector Structure") (HitNormal :type "Vector Structure") (NormalImpulse :type "Vector Structure") (Hit :type "HitResult Structure (by ref)"))
  (bind _health (`self.Health`))
  (bind _asbp_first_person_projectile (cast `/Game/FirstPerson/Blueprints/BP_FirstPersonProjectile` Other))
  (`self.K2_DestroyActor` _asbp_first_person_projectile)
  (`/Engine/EditorBlueprintResources/StandardMacros.DecrementInt` _health
    (:`  `
      (`self.OnHealthChanged`)
      (if (<= _health 0)
        (`/Engine/EditorBlueprintResources/StandardMacros.DoOnce` false
          (:`Completed`
            (bind _returnvalue (`|CreateWidget` "/Game/UI/W_Victory.W_Victory_C" (`GameplayStatics.GetPlayerController` 0)))
            (`UserWidget.AddToViewport` _returnvalue 0)))))))

(fn `UserConstructionScript`)