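; BP_Summoner is a destructible actor that places fish spawners around itself and takes them down when it dies.
; On BeginPlay it spawns BP_FishSpawner actors at random navigable points near its location and stores them in an array.
; Each first-person projectile hit destroys the projectile and decrements Health.
; When Health runs out, a DoOnce gate calls DestroySpawner on each stored spawner in reverse order, then destroys the summoner.
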(event `self.ReceiveBeginPlay`
  (`self.Spawn Spawners`))

(event `Spawn Spawners`
  (for _ (range (`self.SpawnPoints`))
    (bind _randomlocation (`NavigationSystemV1.K2_GetRandomLocationInNavigableRadius` (`self.K2_GetActorLocation`) 500.0 null null))
    (bind _returnvalue (`|SpawnActorFromClass` "/Game/Blueprints/BP_FishSpawner.BP_FishSpawner_C" (`KismetMathLibrary.MakeTransform` _randomlocation) "Undefined" "MultiplyWithRoot" null null))
    (`KismetArrayLibrary.Array_Add` (`self.Spawners`) _returnvalue)))

(event `self.ReceiveHit`
  (params (MyComp :type "PrimitiveComponent Object Reference") (Other :type "Actor Object Reference") (OtherComp :type "PrimitiveComponent Object Reference") (bSelfMoved :type Boolean) (HitLocation :type "Vector Structure") (HitNormal :type "Vector Structure") (NormalImpulse :type "Vector Structure") (Hit :type "HitResult Structure (by ref)"))
  (bind _asbp_first_person_projectile (cast `/Game/FirstPerson/Blueprints/BP_FirstPersonProjectile` Other))
  (`self.K2_DestroyActor` _asbp_first_person_projectile)
  (bind _result (`/Engine/EditorBlueprintResources/StandardMacros.DecrementInt` (`self.Health`))
    (:`  `
      (if (<= _result 0)
        (`/Engine/EditorBlueprintResources/StandardMacros.DoOnce` false
          (:`Completed`
            (bind (_arrayindex _arrayelement) (`/Engine/EditorBlueprintResources/StandardMacros.ReverseForEachLoop` (`self.Spawners`))
              (:`LoopBody`
                (`/Game/Blueprints/BP_FishSpawner.Destroy Spawner` _arrayelement))
              (:`Completed`
                (`self.K2_DestroyActor`)))))))))

(fn `UserConstructionScript`)