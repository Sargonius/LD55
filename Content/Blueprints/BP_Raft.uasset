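; BP_Raft is the player's raft, tracking health and fuel and ending the game when health runs out.
; Damage lowers health, fires the UpdateHealth dispatcher and, at zero or below, runs Death once to show W_GameOver.
; AddFuel and TickFuel change fuel, which UpdateBoatSpeed maps to a speed ratio and broadcasts through UpdateFuel.
; Tick rolls a static mesh at a rate scaled by that speed.
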(event `Damage`
  (params (InDamage :type Integer))
  (bind _output_get (set `self.Health` (- (`self.Health`) InDamage)))
  (`self.UpdateHealth`)
  (if (<= _output_get 0)
    (`/Engine/EditorBlueprintResources/StandardMacros.DoOnce` false
      (:`Completed`
        (`self.Death`)))))

(event `Death`
  (`/Engine/EditorBlueprintResources/StandardMacros.DoOnce` false
    (:`Completed`
      (bind _returnvalue (`|CreateWidget` "/Game/UI/W_GameOver.W_GameOver_C" (`GameplayStatics.GetPlayerController` 0)))
      (`UserWidget.AddToViewport` _returnvalue 0))))

(event `Add Fuel`
  (params (InAmount :type Integer))
  (set `self.CurrentFuel` (+ (`self.CurrentFuel`) InAmount))
  (`self.Update Boat Speed`))

(event `Tick Fuel`
  (`/Engine/EditorBlueprintResources/StandardMacros.DecrementInt` (`self.CurrentFuel`)
    (:`  `
      (`self.Update Boat Speed`))))

(event `Update Boat Speed`
  (bind _output_get (set `self.BoatSpeed` (`KismetMathLibrary.MapRangeUnclamped` (`KismetMathLibrary.Conv_IntToDouble` (`self.CurrentFuel`)) 0.0 (`KismetMathLibrary.Conv_IntToDouble` (`self.MaxFuel`)) 0.0 1.0)))
  (`self.UpdateFuel` _output_get))

(event `self.ReceiveTick`
  (params (DeltaSeconds :type "Float (single-precision)"))
  (`SceneComponent.K2_AddRelativeRotation` (`self.StaticMesh`) (`KismetMathLibrary.MakeRotator` (* DeltaSeconds (`self.RotationSpeedModifier`) (`self.BoatSpeed`))) false false))

(fn `UserConstructionScript`)