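; BP_Summoner is a shootable enemy summoner that places BP_FishSpawner actors at random navigable points around its target location and eases toward that location each tick.
; SpawnFish waits a random delay, plays a cast montage and calls Spawn on BP_SpawnManager.
; Projectile hits reduce Health with a damage montage.
; On death it plays a montage with a timeline-driven vertical offset, destroys its spawners, then removes itself at blend out.
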(event `self.ReceiveBeginPlay`
  (`self.Spawn Spawners`)
  (`KismetSystemLibrary.Delay` 2.0)
  (`GameplayStatics.PlaySoundAtLocation` "/Game/Sound/Spawn_Cue.Spawn_Cue" (`self.TargetLocation`) (struct) 1.0 1.0 0.0 null null null null))

(event `self.ReceiveTick`
  (params (DeltaSeconds :type "Float (single-precision)"))
  (if (!= (`self.TargetLocation`) (`self.K2_GetActorLocation`) :`ErrorTolerance` 10.0)
    (`self.K2_SetActorLocation` (`KismetMathLibrary.VInterpTo` (`self.K2_GetActorLocation`) (`self.TargetLocation`) DeltaSeconds 1.0))))

(event `Spawn Spawners`
  (for _ (range (`self.SpawnPoints`))
    (bind _randomlocation (`NavigationSystemV1.K2_GetRandomLocationInNavigableRadius` (`self.TargetLocation`) 750.0 null null))
    (bind _returnvalue (`|SpawnActorFromClass` "/Game/Blueprints/BP_FishSpawner.BP_FishSpawner_C" (`KismetMathLibrary.MakeTransform` _randomlocation) "Undefined" "MultiplyWithRoot" null null))
    (`KismetArrayLibrary.Array_Add` (`self.Spawners`) _returnvalue)
    (`KismetSystemLibrary.DrawDebugSphere` (`self.K2_GetActorLocation` _returnvalue) 100.0 12 (struct :`R` 1.0 :`B` 0.037368 :`A` 1.0))))

(event `self.ReceiveHit`
  (params (MyComp :type "PrimitiveComponent Object Reference") (Other :type "Actor Object Reference") (OtherComp :type "PrimitiveComponent Object Reference") (bSelfMoved :type Boolean) (HitLocation :type "Vector Structure") (HitNormal :type "Vector Structure") (NormalImpulse :type "Vector Structure") (Hit :type "HitResult Structure (by ref)"))
  (bind _asbp_first_person_projectile (cast `/Game/FirstPerson/Blueprints/BP_FirstPersonProjectile` Other))
  (`self.Deal Damage` (`/Game/FirstPerson/Blueprints/BP_FirstPersonProjectile.Damage` _asbp_first_person_projectile))
  (`self.K2_DestroyActor` _asbp_first_person_projectile))

(event `Deal Damage`
  (params (InDamage :type Integer))
  (bind _health (`self.Health`))
  (if (> _health 0)
    (set `self.Health` (- _health InDamage))
    (if (<= (`self.Health`) 0)
      (`/Engine/EditorBlueprintResources/StandardMacros.DoOnce` false
        (:`Completed`
          (`|PlayMontage` (`self.SkeletalMesh`) "/Game/Blender_Res/Summon/A_S_Die_Montage.A_S_Die_Montage"
            (:`then`
              (`|ExecutionSequence`
                (:`then_0`
                  (bind (_direction _newtrack_0) (`Timeline|Timeline` :!via `PlayFromStart`)
                    (:`Update`
                      (`self.K2_AddActorWorldOffset` (`KismetMathLibrary.MakeVector` 0.0 0.0 _newtrack_0)))))
                (:`then_1`
                  (bind (_arrayindex _arrayelement) (`/Engine/EditorBlueprintResources/StandardMacros.ReverseForEachLoop` (`self.Spawners`))
                    (:`LoopBody`
                      (`/Game/Blueprints/BP_FishSpawner.Destroy Spawner` _arrayelement))))))
            (:`OnBlendOut`
              (`self.K2_DestroyActor`)))))
      (else
        (`|PlayMontage` (`self.SkeletalMesh`) "/Game/Blender_Res/Summon/A_S_Damage_Montage.A_S_Damage_Montage")))))

(event `Spawn Fish`
  (`KismetSystemLibrary.Delay` (`KismetMathLibrary.RandomFloatInRange` 1.0 3.0))
  (`|PlayMontage` null "/Game/Blender_Res/Summon/A_S_Cast_Montage.A_S_Cast_Montage"
    (:`then`
      (bind _returnvalue (`GameplayStatics.GetActorOfClass` "/Game/Blueprints/BP_SpawnManager.BP_SpawnManager_C"))
      (`/Game/Blueprints/BP_SpawnManager.Spawn` _returnvalue))))

(fn `UserConstructionScript`)