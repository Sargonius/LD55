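; BP_Junk is a drifting pickup that grants the first-person character a bonus when collected.
; It picks a random speed on BeginPlay and moves along its forward vector each tick, pausing while attached to another actor.
; When its sphere overlaps the character's capsule, ApplyBonus passes BonusType to the character found by class lookup.
; The junk then tells the overlapping character to detach its harpooned item and destroys itself.
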(event `self.ReceiveBeginPlay`
  (set `self.Speed` (`KismetMathLibrary.RandomFloatInRange` 50.0 175.0)))

(event `self.ReceiveTick`
  (params (DeltaSeconds :type "Float (single-precision)"))
  (`/Engine/EditorBlueprintResources/StandardMacros.IsValid` (`self.GetAttachParentActor`)
    (:`Is Not Valid`
      (`self.K2_AddActorWorldOffset` (* (`self.GetActorForwardVector`) (* DeltaSeconds (`self.Speed`)))))))

(event `self.Sphere.OnComponentBeginOverlap`
  (params (OverlappedComponent :type "PrimitiveComponent Object Reference") (OtherActor :type "Actor Object Reference") (OtherComp :type "PrimitiveComponent Object Reference") (OtherBodyIndex :type Integer) (bFromSweep :type Boolean) (SweepResult :type "HitResult Structure (by ref)"))
  (bind _asbp_first_person_character (cast `/Game/FirstPerson/Blueprints/BP_FirstPersonCharacter` OtherActor))
  (cast `CapsuleComponent` OtherComp)
  (`self.Apply Bonus`)
  (`/Game/FirstPerson/Blueprints/BP_FirstPersonCharacter.Detach Item From Harpoon` _asbp_first_person_character)
  (`self.K2_DestroyActor`))

(event `Apply Bonus`
  (bind _returnvalue (`GameplayStatics.GetActorOfClass` "/Game/FirstPerson/Blueprints/BP_FirstPersonCharacter.BP_FirstPersonCharacter_C"))
  (`/Game/FirstPerson/Blueprints/BP_FirstPersonCharacter.Add Bonus` _returnvalue (`self.BonusType`)))

(fn `UserConstructionScript`)