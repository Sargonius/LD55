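; BP_BossFishSpawner spawns a BP_Fish at its own transform as the boss loses health.
; On BeginPlay it finds BP_Boss and binds to its health-changed event.
; Each change checks three descending health thresholds, each gated by a DoOnce so it fires only once.
; All three feed one shared short random Delay before the spawn, so thresholds crossed during a pending delay yield a single fish.
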(event `self.ReceiveBeginPlay`
  (bind _returnvalue (`GameplayStatics.GetActorOfClass` "/Game/Blueprints/BP_Boss.BP_Boss_C"))
  (add `/Game/Blueprints/BP_Boss.OnHealthChanged` _returnvalue (delegate `Handle Boss Health Change`)))

(event `Handle Boss Health Change`
  (bind _returnvalue (`GameplayStatics.GetActorOfClass` "/Game/Blueprints/BP_Boss.BP_Boss_C"))
  (`|ExecutionSequence`
    (:`then_0`
      (bind _health (`/Game/Blueprints/BP_Boss.Health` _returnvalue))
      (if (<= _health 150)
        (`/Engine/EditorBlueprintResources/StandardMacros.DoOnce` false
          (:`Completed`
            (`KismetSystemLibrary.Delay` (`KismetMathLibrary.RandomFloatInRange` 0.2 1.0) :!label _label)
            (`|SpawnActorFromClass` "/Game/Blueprints/BP_Fish.BP_Fish_C" (`self.GetTransform`) "Undefined" "MultiplyWithRoot" null null)))))
    (:`then_1`
      (if (<= _health 100)
        (`/Engine/EditorBlueprintResources/StandardMacros.DoOnce` false
          (:`Completed`
            (goto _label)))))
    (:`then_2`
      (if (<= _health 50)
        (`/Engine/EditorBlueprintResources/StandardMacros.DoOnce` false
          (:`Completed`
            (goto _label)))))))

(fn `UserConstructionScript`)